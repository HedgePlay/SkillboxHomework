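; BP_TrafficLightsManager cycles every BP_TraffictLight actor in the level through three color states in unison.
; From BeginPlay, the Recolor event gathers the lights with GetAllActorsOfClass and calls ChangeColor on them, separated by fixed Delays of differing length.
; Each color comes from an enum-keyed map in ColorSettings, and Recolor calls itself after the last Delay to loop indefinitely.
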(event `self.ReceiveBeginPlay`
  (`self.Recolor`))

(event `Recolor`
  (bind _colorsettings_colormap (break `/Game/Blueprints/S_LIghtColor` (`self.ColorSettings`)))
  (bind _colorsettings_colormap_2 (break `/Game/Blueprints/S_LIghtColor` (`self.ColorSettings`)))
  (bind _colorsettings_colormap_3 (break `/Game/Blueprints/S_LIghtColor` (`self.ColorSettings`)))
  (bind _outactors (`GameplayStatics.GetAllActorsOfClass` "/Game/Blueprints/BP_TraffictLight.BP_TraffictLight_C"))
  (`/Game/Blueprints/BP_TraffictLight.ChangeColor` _outactors (`BlueprintMapLibrary.Map_Find` _colorsettings_colormap "NewEnumerator0"))
  (`KismetSystemLibrary.Delay` 5.0)
  (`/Game/Blueprints/BP_TraffictLight.ChangeColor` _outactors (`BlueprintMapLibrary.Map_Find` _colorsettings_colormap_2 "NewEnumerator1"))
  (`KismetSystemLibrary.Delay` 1.0)
  (`/Game/Blueprints/BP_TraffictLight.ChangeColor` _outactors (`BlueprintMapLibrary.Map_Find` _colorsettings_colormap_3 "NewEnumerator2"))
  (`KismetSystemLibrary.Delay` 2.0)
  (`self.Recolor`))

(fn `UserConstructionScript`)